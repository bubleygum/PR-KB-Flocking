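; BP_Flock2 is a work-in-progress boids-style flock manager that calculates cohesion, alignment and separation data over its Members array.
; Cohesion averages overlap locations from each BP_Cone's Sphere, additionally dividing each by neighbor count.
; Alignment averages member velocities, while separation only stores offsets from each cone's Box overlaps.
; Averages are printed but never applied to movement, and nothing live in this graph calls these events.
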(event `self.ReceiveTick`
  (params (DeltaSeconds :type "Float (single-precision)")))

(event `self.ReceiveBeginPlay`)

(event `calAvgLoc`
  (bind _combineloc (`self.combineLoc`))
  (bind _combinelocindex (`self.combineLocIndex`))
  ;[1 1 1] Cari avg loc tiap cone buat cohesion | avgLoc = target Loc
  (for _array_element (`self.members`)
    (bind _asbp_cone (cast `/Game/Kerucut/BP_Cone` _array_element))
    (bind _overlappingactors (`PrimitiveComponent.GetOverlappingActors` (`/Game/Kerucut/BP_Cone.Sphere` _asbp_cone) null))
    (bind _returnvalue (`GameplayStatics.GetActorArrayAverageLocation` _overlappingactors))
    (`KismetArrayLibrary.Array_Set` _combineloc _combinelocindex (/ _returnvalue (`KismetArrayLibrary.Array_Length` _overlappingactors)) true)
    (bind _result (`/Engine/EditorBlueprintResources/StandardMacros.IncrementInt` _combinelocindex)
      (:`  `
        (set `self.combineLocIndex` _result))))
  (bind _output_get (set `self.avgLoc` (`KismetMathLibrary.GetVectorArrayAverage` _combineloc)))
  (`KismetSystemLibrary.PrintString` (`KismetStringLibrary.Conv_VectorToString` _output_get)))

(event `calAvgAlign`
  (bind _com_vel_index (`self.com Vel Index`))
  ;[1 1 1] get avg velocity of each member in flock
  (for _array_element (`self.members`)
    (`KismetArrayLibrary.Array_Set` (`self.countVel`) _com_vel_index (`self.GetVelocity` _array_element) true)
    (bind _result (`/Engine/EditorBlueprintResources/StandardMacros.IncrementInt` _com_vel_index)
      (:`  `
        (set `self.com Vel Index` _result))))
  (for (_array_element_2 _array_index) (`self.countVel`)
    (set `self.comVel` (+ _array_element_2 (`self.comVel`))))
  (bind _output_get (set `self.avgVel` (/ (`self.comVel`) _array_index)))
  (`KismetSystemLibrary.PrintString` (`KismetStringLibrary.Conv_VectorToString` _output_get)))

(event `calSeparation`
  (bind _sepvecindex (`self.sepVecIndex`))
  (for _array_element (`self.members`)
    (bind _asbp_cone (cast `/Game/Kerucut/BP_Cone` _array_element))
    (bind _output_get (set `self.neighborBP` (`PrimitiveComponent.GetOverlappingActors` (`/Game/Kerucut/BP_Cone.Box` _asbp_cone) null)))
    (for _array_element_2 _output_get
      (`KismetArrayLibrary.Array_Set` (`self.seVec`) _sepvecindex (- (`self.K2_GetActorLocation` _array_element) (`self.K2_GetActorLocation` _array_element_2)) true)
      (bind _result (`/Engine/EditorBlueprintResources/StandardMacros.IncrementInt` _sepvecindex)
        (:`  `
          (set `self.sepVecIndex` _result))))))

(fn `UserConstructionScript`)