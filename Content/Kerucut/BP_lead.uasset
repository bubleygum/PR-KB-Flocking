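; BP_lead is an unfinished actor Blueprint with a capsule component, apparently prototyping random wandering movement.
; Its getrandloc event stores the actor location plus a small random offset in NewLoc, but nothing live calls it.
; Tick and MoveToRandLoc are empty.
; Disconnected fragments hold delayed debug prints and capsule moves toward NewLoc or a BP_ConeChar average location scaled by MaxDistance, so none of them run.
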(event `MoveToRandLoc`)

(event `self.ReceiveTick`
  (params (DeltaSeconds :type "Float (single-precision)")))

(event `get rand loc`
  (bind _returnvalue (`KismetMathLibrary.RandomFloatInRange` -3.0 3.0))
  (set `self.newLoc` (+ (`self.K2_GetActorLocation`) (`KismetMathLibrary.MakeVector` _returnvalue _returnvalue _returnvalue))))

(fn `UserConstructionScript`)