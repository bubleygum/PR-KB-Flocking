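; BP_ConePawn is an unfinished flocking pawn that finds neighbors through its Sphere overlaps.
; calAvgLoc averages overlapping cone locations into AvgLoc for cohesion, and calAvgVelo averages overlapping actors' velocities, but neither is called here.
; Tick calls CalAvgVelo2, whose loop is empty, then after a half-second Delay issues AIMoveTo toward AvgLoc and prints on success.
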(event `self.ReceiveBeginPlay`)

(event `self.ReceiveTick`
  (params (DeltaSeconds :type "Float (single-precision)"))
  (`self.cal avg velo2`)
  (`KismetSystemLibrary.Delay` 0.5)
  (`|AIMoveTo` self (`self.avg loc`) null
    (:`OnSuccess`
      (`KismetSystemLibrary.PrintString` "Hello"))))

(event `calAvgLoc`
  ;[1 1 1] Cari avg loc tiap cone buat cohesion | avgLoc = target Loc
  (bind _returnvalue (`GameplayStatics.GetActorArrayAverageLocation` (`PrimitiveComponent.GetOverlappingActors` (`self.Sphere`) "BP_ConePawn_C")))
  (bind _output_get (set `self.avg loc` _returnvalue))
  (`KismetSystemLibrary.PrintString` (`KismetStringLibrary.Conv_VectorToString` _output_get)))

(event `calAvgVelo`
  (bind _com_vel_index (`self.com vel index`))
  ;[1 1 1] get avg velocity of each member in flock
  (for _array_element (`PrimitiveComponent.GetOverlappingActors` (`self.Sphere`) null)
    (`KismetArrayLibrary.Array_Set` (`self.count vel`) _com_vel_index (`self.GetVelocity` _array_element) true)
    (bind _result (`/Engine/EditorBlueprintResources/StandardMacros.IncrementInt` _com_vel_index)
      (:`  `
        (set `self.com vel index` _result))))
  (for (_array_element_2 _array_index) (`self.count vel`)
    (set `self.com vel` (+ _array_element_2 (`self.com vel`))))
  (bind _output_get (set `self.avg vel` (/ (`self.com vel`) _array_index)))
  (`KismetSystemLibrary.PrintString` (`KismetStringLibrary.Conv_VectorToString` _output_get)))

(event `cal avg velo2`
  (for _array_element (`PrimitiveComponent.GetOverlappingActors` (`self.Sphere`) null)
    _))

(fn `UserConstructionScript`)