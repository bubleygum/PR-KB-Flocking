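; BP_ConeChar is a flocking cone character that computes boid-style cohesion, alignment and avoidance values.
; Each Tick stores the average location of all cones and an average velocity from SphereRadius neighbours, using accumulators that never reset here.
; Separation, rotation, random-location and navmesh-path avoidance events exist but are not called within this Blueprint.
; Overlapping a BP_Sphere only adds zero movement input and prints a debug message.
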(event `self.ReceiveTick`
  (params (DeltaSeconds :type "Float (single-precision)"))
  ;[1 1 1] AI move to jalan
  (`self.calAvgLoc`)
  (`self.calAvgVelo`))

(event `calAvgLoc`
  ;[1 1 1] Cari avg loc tiap cone buat cohesion | avgLoc = target Loc
  (bind _outactors (`GameplayStatics.GetAllActorsOfClass` "BP_ConeChar_C"))
  (bind _returnvalue (`GameplayStatics.GetActorArrayAverageLocation` _outactors))
  (set `self.avg loc` _returnvalue))

(event `cohesion2`
  ;[1 1 1] Cari avg loc tiap cone buat cohesion | avgLoc = target Loc
  (bind _returnvalue (`GameplayStatics.GetActorArrayAverageLocation` (`PrimitiveComponent.GetOverlappingActors` (`self.Sphere Radius`) "BP_ConeChar_C")))
  (set `self.avg loc` _returnvalue))

(event `calAvgVelo`
  (bind _com_vel_index (`self.com vel index`))
  ;[1 1 1] get avg velocity of each member in flock
  (for _array_element (`PrimitiveComponent.GetOverlappingActors` (`self.Sphere Radius`) "BP_ConeChar_C")
    (`KismetArrayLibrary.Array_Set` (`self.count vel`) _com_vel_index (`self.GetVelocity` _array_element) true)
    (bind _result (`/Engine/EditorBlueprintResources/StandardMacros.IncrementInt` _com_vel_index)
      (:`  `
        (set `self.com vel index` _result))))
  (for _array_element_2 (`self.count vel`)
    (set `self.com vel` (+ _array_element_2 (`self.com vel`))))
  (set `self.avg vel` (/ (`self.com vel`) (`self.com vel index`))))

(event `avoid`
  (bind _returnvalue (`self.K2_GetActorLocation`))
  (bind _returnvalue_2 (`self.K2_GetActorRotation`))
  (if (> (`KismetArrayLibrary.Array_Length` (`PrimitiveComponent.GetOverlappingActors` (`self.Sphere avoid`) "/Game/Kerucut/BP_Sphere.BP_Sphere_C")) 0)
    (bind _returnvalue_3 (`NavigationSystemV1.FindPathToLocationSynchronously` _returnvalue (`self.avg loc`) null null))
    (for _array_element (`NavigationPath.PathPoints` _returnvalue_3)
      (bind (_returnvalue_roll _returnvalue_pitch _returnvalue_yaw) (`KismetMathLibrary.BreakRotator` (`KismetMathLibrary.FindLookAtRotation` (`KismetMathLibrary.Conv_RotatorToVector` _returnvalue_2) (- _returnvalue _array_element))))
      (`self.K2_SetActorRotation` (`KismetMathLibrary.RInterpTo` _returnvalue_2 (`KismetMathLibrary.MakeRotator` 0.0 0.0 _returnvalue_yaw)))
      (set `self.avg loc` _array_element)
      (`KismetSystemLibrary.Delay` 1.0))))

(event `cal separation`
  (bind _min (`self.min`))
  (bind _returnvalue (`GameplayStatics.GetActorArrayAverageLocation` (`PrimitiveComponent.GetOverlappingActors` (`self.Sphere Radius`) "BP_ConeChar_C")))
  (set `self.sepparation` (* _returnvalue (`KismetMathLibrary.MakeVector` _min _min))))

(event `rotate`
  (`self.K2_SetActorRotation` (`KismetMathLibrary.FindLookAtRotation` (`KismetMathLibrary.Conv_RotatorToVector` (`self.K2_GetActorRotation`)) (`self.sepparation`))))

(event `rand loc`
  (bind (_avg_loc_x _avg_loc_y) (`KismetMathLibrary.BreakVector` (`self.avg loc`)))
  (if (<= _avg_loc_x 0.0)
    (set `self.ranLoc` (`KismetMathLibrary.MakeVector` (+ _avg_loc_x 100.0)))
    (else
      (set `self.ranLoc` (`KismetMathLibrary.MakeVector` (- _avg_loc_x 100.0)))))
  (if (<= _avg_loc_y 0.0)
    (set `self.ranLoc` (`KismetMathLibrary.MakeVector` 0.0 (+ _avg_loc_y 100.0)))
    (else
      (set `self.ranLoc` (`KismetMathLibrary.MakeVector` 0.0 (- _avg_loc_y 100.0))))))

(event `self.ReceiveActorBeginOverlap`
  (params (OtherActor :type "Actor Object Reference"))
  (bind _asbp_sphere (cast `/Game/Kerucut/BP_Sphere` OtherActor))
  (if (`self.IsOverlappingActor` _asbp_sphere)
    (`self.AddMovementInput` (0.0 0.0 0.0))
    (`KismetSystemLibrary.PrintString` "avoid 2")))

(fn `UserConstructionScript`)