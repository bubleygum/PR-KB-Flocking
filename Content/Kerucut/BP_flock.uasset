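; BP_flock is a flock manager that computes average location and velocity over its FlockMembers array.
; updateFlock runs calculateLoc once per member, each time storing and printing the whole group's average location.
; calculateVel copies member velocities into MemVal, re-summing that array inside the member loop to derive and print NewVel, without resetting the sum or index.
; Nothing here calls updateFlock or calculateVel, or moves the members.
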(event `self.ReceiveBeginPlay`)

(event `updateFlock`
  (for _ (`self.flockMembers`)
    (`self.calculateLoc`)))

(event `calculateLoc`
  (bind _returnvalue (`GameplayStatics.GetActorArrayAverageLocation` (`self.flockMembers`)))
  (bind _output_get (set `self.newLoc` _returnvalue))
  (`KismetSystemLibrary.PrintString` (`KismetStringLibrary.Conv_VectorToString` _output_get)))

(event `calculateVel`
  (bind _memval (`self.memVal`))
  (bind _index (`self.Index`))
  (for _array_element (`self.flockMembers`)
    (`KismetArrayLibrary.Array_Set` _memval _index (`self.GetVelocity` _array_element))
    (bind _result (`/Engine/EditorBlueprintResources/StandardMacros.IncrementInt` _index)
      (:`  `
        (bind _output_get (set `self.Index` _result))
        (for _array_element_2 _memval
          (bind _output_get_2 (set `self.combineVel` (+ _array_element_2 (`self.combineVel`))))
          (bind _output_get_3 (set `self.newVel` (/ _output_get_2 _output_get)))
          (`KismetSystemLibrary.PrintString` (`KismetStringLibrary.Conv_VectorToString` _output_get_3)))))))

(fn `UserConstructionScript`)